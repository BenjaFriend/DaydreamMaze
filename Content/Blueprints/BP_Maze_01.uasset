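; BP_Maze_01 is a tilt maze actor for a Daydream VR ball game, steered by the motion controller.
; Each tick it copies the controller rotation from BP_GVRPawn onto its own rotation.
; The pawn's spawn event makes it replace any existing BP_Ball with a new one at BallSpawnPoint.
; A ball overlapping the goal is destroyed and triggers win particles there.
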(event `self.ReceiveBeginPlay`
  (bind _asbp_gvrpawn (cast `/Game/Blueprints/BP_GVRPawn` (`GameplayStatics.GetPlayerPawn` 0)))
  (bind _output_get (set `self.Player Pawn` _asbp_gvrpawn))
  (add `/Game/Blueprints/BP_GVRPawn.SpawnNewBallEvent` _output_get (delegate `SpawnNewBall`)))

(event `SpawnNewBall`
  (bind _currentball (`self.CurrentBall`))
  ;[1 1 1] If there is already a ball, destroy it
  (if (`KismetSystemLibrary.IsValid` _currentball)
    (`self.K2_DestroyActor` _currentball))
  ;[1 1 1] Spawn  a new ball at the spawn point
  (bind _returnvalue (`|SpawnActorFromClass` "/Game/Blueprints/BP_Ball.BP_Ball_C" (`SceneComponent.K2_GetComponentToWorld` (`self.Ball Spawn Point`)) "Undefined" "OverrideRootScale" null null))
  (set `self.CurrentBall` _returnvalue))

(event `self.ReceiveTick`
  (params (DeltaSeconds :type "Float (single-precision)"))
  (bind _player_pawn (`self.Player Pawn`))
  ;[1 1 1] Rotate the maze based on the daydream controller
  (if (`KismetSystemLibrary.IsValid` _player_pawn)
    (`self.K2_SetActorRotation` (`/Game/Blueprints/BP_GVRPawn.Controller Rotation` _player_pawn))))

(event `self._Goal.OnComponentBeginOverlap`
  (params (OverlappedComponent :type "PrimitiveComponent Object Reference") (OtherActor :type "Actor Object Reference") (OtherComp :type "PrimitiveComponent Object Reference") (OtherBodyIndex :type Integer) (bFromSweep :type Boolean) (SweepResult :type "HitResult Structure (by ref)"))
  ;[1 1 1] Detect when the ball hits the maze
  (bind _asbp_ball (cast `/Game/Blueprints/BP_Ball` OtherActor))
  (`self.K2_DestroyActor` _asbp_ball)
  (`GameplayStatics.SpawnEmitterAtLocation` "/Game/P_WinParticles.P_WinParticles" (`SceneComponent.K2_GetComponentLocation` (`self._Goal`))))

(fn `UserConstructionScript`)